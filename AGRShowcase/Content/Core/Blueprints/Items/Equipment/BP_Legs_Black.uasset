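; BP_Legs_Black is a leg equipment item that boosts its wearer's sprint speed while equipped.
; It binds the equip and unequip events of its BPC_AGR_ItemCore component, adding a fixed bonus on equip and subtracting it on unequip.
; Sprint speed is read and written on the inventory component's owner through message calls, so the change is relative to the current value.
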(event OnItemEquipped(BPC_AGR_ItemCore)
  (params (InventoryComponent :type AGR%20Inventory%20Component%20Object%20Reference) (EquipmentSlot :type Gameplay%20Tag%20Structure%20%28by%20ref%29))
  (bind _returnvalue (Components|GetOwner InventoryComponent))
  (bind _sprintspeed (Class|BPICharacter|GetSprintSpeed(Message) _returnvalue))
  (Class|BPICharacter|SetSprintSpeed(Message) _returnvalue (+ _sprintspeed 8e+02)))

(event OnItemUnequipped(BPC_AGR_ItemCore)
  (params (InventoryComponent :type AGR%20Inventory%20Component%20Object%20Reference) (EquipmentSlot :type Gameplay%20Tag%20Structure%20%28by%20ref%29))
  (bind _returnvalue (Components|GetOwner InventoryComponent))
  (bind _sprintspeed (Class|BPICharacter|GetSprintSpeed(Message) _returnvalue))
  (Class|BPICharacter|SetSprintSpeed(Message) _returnvalue (+ _sprintspeed -8e+02)))

(event EventBeginPlay
  (|CallParentFunction) ; This node is disabled and will not be called.\nDrag off pins to build functionality.
)

(event Collision|EventActorBeginOverlap
  (params (OtherActor :type Actor%20Object%20Reference))
  (|CallParentFunction OtherActor) ; This node is disabled and will not be called.\nDrag off pins to build functionality.
)

(event EventTick
  (params (DeltaSeconds :type Float%20%28single-precision%29))
  (|CallParentFunction DeltaSeconds) ; This node is disabled and will not be called.\nDrag off pins to build functionality.
)

(fn ConstructionScript
  (|CallParentFunction))