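; BP_MasterItem is an item Blueprint, named as the master, that defines default permission rules for inventory actions.
; Its checks read the BPCAGRItemCore component: pickup requires an empty owner ID, and equipping requires a non-exact gameplay tag match against the equipable slots.
; Destroy, drop and unequip are always allowed, while use is always refused.
; The event graph and construction script are empty.
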(event EventBeginPlay)

(event Collision|EventActorBeginOverlap
  (params (OtherActor :type Actor%20Object%20Reference)))

(event EventTick
  (params (DeltaSeconds :type Float%20%28single-precision%29)))

(fn ConstructionScript)

(fn CanItembeDestroyed
  (params (InventoryComponent :type AGR%20Inventory%20Component%20Object%20Reference))
  (return true))

(fn CanItembeDropped
  (params (InventoryComponent :type AGR%20Inventory%20Component%20Object%20Reference))
  (return true))

(fn CanItembeEquipped
  (params (InventoryComponent :type AGR%20Inventory%20Component%20Object%20Reference) (Slot :type Gameplay%20Tag%20Structure))
  (return (GameplayTags|HasTag (Variables|/Game/Core/Blueprints/Components/BPC_AGR_ItemCore.BPC_AGR_ItemCore_C|GetEquipableSlots (Variables|Default|GetBPC_AGR_ItemCore)) Slot)))

(fn CanItembePickedUp
  (params (InventoryComponent :type AGR%20Inventory%20Component%20Object%20Reference))
  (return (Utilities|Array|IsEmpty (Class|AGRItemComponent|GetOwnerID (Variables|Default|GetBPC_AGR_ItemCore)))))

(fn CanItembeUnequipped
  (params (InventoryComponent :type AGR%20Inventory%20Component%20Object%20Reference) (Slot :type Gameplay%20Tag%20Structure))
  (return true))

(fn CanItembeUsed
  (params (InventoryComponent :type AGR%20Inventory%20Component%20Object%20Reference) (ActionType :type Gameplay%20Tag%20Structure))
  (return false))