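; BP_MasterHandEquipment is a hand equipment item, apparently a base class, that attaches to its owner's skeletal mesh when equipped.
; It responds to the OnItemEquipped event of BPC_AGR_ItemCore and finds the first skeletal mesh tagged MainMesh on the inventory component's owner.
; If that mesh is valid, it snaps to the left socket for the LeftHand slot, or the right socket for any other slot.
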(event OnItemEquipped(BPC_AGR_ItemCore)
  (params (InventoryComponent :type AGR%20Inventory%20Component%20Object%20Reference) (EquipmentSlot :type Gameplay%20Tag%20Structure%20%28by%20ref%29))
  (bind _returnvalue (Components|GetOwner InventoryComponent))
  (bind _returnvalue_2 (Actor|GetComponentsbyTag _returnvalue "/Script/Engine.SkeletalMeshComponent" "MainMesh"))
  (bind _output (Utilities|Array|Get(acopy) _returnvalue_2))
  (Utilities|IsValid _output
    (:Is%20Valid
      (Transformation|AttachComponentToComponent _output (select (== EquipmentSlot "(TagName=\"EquipmentSlot.LeftHand\")") (Variables|Default|GetEquipSocketLeft) (Variables|Default|GetEquipSocketRight)) "SnapToTarget" "SnapToTarget" "SnapToTarget" true))))

(event EventBeginPlay
  (|CallParentFunction) ; This node is disabled and will not be called.\nDrag off pins to build functionality.
)

(event Collision|EventActorBeginOverlap
  (params (OtherActor :type Actor%20Object%20Reference))
  (|CallParentFunction OtherActor) ; This node is disabled and will not be called.\nDrag off pins to build functionality.
)

(event EventTick
  (params (DeltaSeconds :type Float%20%28single-precision%29))
  (|CallParentFunction DeltaSeconds) ; This node is disabled and will not be called.\nDrag off pins to build functionality.
)

(fn ConstructionScript
  (|CallParentFunction))