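; Inventory component Blueprint that carries server-side item actions, with the equip event noted as called from client widgets.
; SVR_EquipItem equips an item visibly into a slot or unequips it, through the item actor's item component.
; SVR_DropItem drops an item through that same component, at a transform calculated a short distance away for that item.
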(event Custom|SVR_EquipItem
  (params (Actor :type Actor%20Object%20Reference) (Slot :type Gameplay%20Tag%20Structure) (Unequip :type Boolean))
  (bind _returnvalue (Class|AGRInventoryFunctionLibrary|GetItemComponent Actor))
  (bind _self self)
  ;[1 1 1] Calling this Server event from Client widgets
  (if Unequip
    (Class|AGRItemComponent|UnequipItem _returnvalue _self Slot)
    (else
      (Class|AGRItemComponent|EquipItem _returnvalue _self Slot true))))

(event Custom|SVR_DropItem
  (params (Actor :type Actor%20Object%20Reference))
  (bind _returnvalue (Class|AGRInventoryComponent|CalculateDropTransform Actor 5e+01))
  (bind (_location _rotation) (Math|Transform|BreakTransform _returnvalue))
  (Class|AGRItemComponent|DropItem (Class|AGRInventoryFunctionLibrary|GetItemComponent Actor) self _location _rotation true))

(event EventBeginPlay)

(event EventTick
  (params (DeltaSeconds :type Float%20%28single-precision%29)))