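; BFL_AGR is a function library of typed lookup helpers for the AGR inventory and item components and the player HUD.
; GetInventoryCore and GetItemCore fetch the input's component and cast it to the project's BPC_AGR core classes.
; GetHUD accepts a PlayerController or a Pawn controlled by one and returns its BP_PlayerHUD.
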(fn GetInventoryCore
  (params (Input :type Actor%20Object%20Reference))
  (bind _asbpc_agr_inventory_core (Utilities|Casting|CastToBPC_AGR_InventoryCore (Class|AGRInventoryFunctionLibrary|GetInventoryComponent Input)))
  (return _asbpc_agr_inventory_core))

(fn GetItemCore
  (params (Input :type Actor%20Object%20Reference))
  (bind _asbpc_agr_item_core (Utilities|Casting|CastToBPC_AGR_ItemCore (Class|AGRInventoryFunctionLibrary|GetItemComponent Input)))
  (return _asbpc_agr_item_core))

(fn GetHUD
  (params (Actor :type Actor%20Object%20Reference))
  (bind _asplayer_controller (Utilities|Casting|CastToPlayerController Actor)
    (:then
      (LocalVariables|SetController _asplayer_controller))
    (:CastFailed
      (bind _aspawn (Utilities|Casting|CastToPawn Actor))
      (bind _asplayer_controller_2 (Utilities|Casting|CastToPlayerController (Pawn|GetController _aspawn)))
      (LocalVariables|SetController _asplayer_controller_2)))
  (bind _asbp_player_hud (Utilities|Casting|CastToBP_PlayerHUD (HUD|GetHUD (LocalVariables|GetController))))
  (return _asbp_player_hud))