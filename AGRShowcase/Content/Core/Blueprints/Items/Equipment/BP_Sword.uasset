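; Sword equipment item that drives the owner's weapon-stance animation through the AGR item core component's equip and unequip events.
; Equipping opens the LeftHand slot on the item and sets a two-handed pose for that slot, or one-handed otherwise.
; Unequipping from RightHand closes the LeftHand slot, unequips it and resets the locomotion pose; any other slot returns to the one-handed pose.
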(event OnItemEquipped(BPC_AGR_ItemCore)
  (params (InventoryComponent :type AGR%20Inventory%20Component%20Object%20Reference) (EquipmentSlot :type Gameplay%20Tag%20Structure%20%28by%20ref%29))
  (GameplayTags|AddGameplayTag (Variables|/Game/Core/Blueprints/Components/BPC_AGR_ItemCore.BPC_AGR_ItemCore_C|GetEquipableSlots (Variables|Default|GetBPC_AGR_ItemCore)) "(TagName=\"EquipmentSlot.LeftHand\")" :!class /Script/GameplayTags.BlueprintGameplayTagLibrary)
  (Class|AGRLocomotionComponent|SetPose (Class|AGRAnimationFunctionLibrary|GetLocomotionComponent (Components|GetOwner InventoryComponent)) (GameplayTags|MakeLiteralGameplayTag (select (== EquipmentSlot "(TagName=\"EquipmentSlot.LeftHand\")") "(TagName=\"States.Animation.2HandedSword\")" "(TagName=\"States.Animation.1HandedSword\")"))))

(event OnItemUnequipped(BPC_AGR_ItemCore)
  (params (InventoryComponent :type AGR%20Inventory%20Component%20Object%20Reference) (EquipmentSlot :type Gameplay%20Tag%20Structure%20%28by%20ref%29))
  (bind _returnvalue (Components|GetOwner InventoryComponent))
  (bind _returnvalue_2 (Class|AGRAnimationFunctionLibrary|GetLocomotionComponent _returnvalue))
  (if (== EquipmentSlot "(TagName=\"EquipmentSlot.RightHand\")")
    (GameplayTags|RemoveGameplayTag (Variables|/Game/Core/Blueprints/Components/BPC_AGR_ItemCore.BPC_AGR_ItemCore_C|GetEquipableSlots (Variables|Default|GetBPC_AGR_ItemCore)) "(TagName=\"EquipmentSlot.LeftHand\")" :!class /Script/GameplayTags.BlueprintGameplayTagLibrary)
    (Class|AGRItemComponent|UnequipItem (Variables|Default|GetBPC_AGR_ItemCore) InventoryComponent "(TagName=\"EquipmentSlot.LeftHand\")")
    (Class|AGRLocomotionComponent|SetPose _returnvalue_2)
    (else
      (Class|AGRLocomotionComponent|SetPose _returnvalue_2 "(TagName=\"States.Animation.1HandedSword\")"))))

(event EventBeginPlay
  (|CallParentFunction) ; This node is disabled and will not be called.\nDrag off pins to build functionality.
)

(event Collision|EventActorBeginOverlap
  (params (OtherActor :type Actor%20Object%20Reference))
  (|CallParentFunction OtherActor) ; This node is disabled and will not be called.\nDrag off pins to build functionality.
)

(event EventTick
  (params (DeltaSeconds :type Float%20%28single-precision%29))
  (|CallParentFunction DeltaSeconds) ; This node is disabled and will not be called.\nDrag off pins to build functionality.
)

(fn ConstructionScript
  (|CallParentFunction))